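; BPC_Stats is an actor component that holds a Health stat for its owner.
; IncreaseStats switches on a stat type and adds the passed value to Health, clamped between zero and MaxHealth.
; Its zero-health check leads to no action; a separate Die event forwards DieMessage to the owning actor but is not called within this component.
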(event `Die`
  (message `/Game/Abno_Punchers/Main_Blueprints/BPI_Damage.Die` (`self.GetOwner`)))

(fn `Increase_Stats`
  (params (Stats :type "/Game/Abno_Punchers/Main_Blueprints/E_Stats Enum" :default "NewEnumerator0") (Vcalue :type "Float (double-precision)"))
  (switch `/Game/Abno_Punchers/Main_Blueprints/E_Stats` Stats
    (:`NewEnumerator0`
      (set `self.Health` (`KismetMathLibrary.FClamp` (+ (`self.Health`) Vcalue) 0.0 (`self.Max Health`)))
      (`|ExecutionSequence`
        (:`then_0`
          (if (<= (`self.Health`) 0.0)
            _))))))